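; BP_Hero is the player's 2D side-scrolling character, with basic, heavy and thunder-spawning ranged attacks, double jump and hold-to-run dash.
; Input and movement events jump the sprite's animation state machine to named nodes.
; Attacks and landing set a movement lock, never cleared here, that gates walking and left/right facing.
; Damage updates the health bar through CallChangingHealth and knocks the hero away from EnemyPositionX, or respawns it at its start location on death.
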(event Custom|Respawn
  (Default|CallChangingHealth 0.0)
  (Transformation|SetActorLocation (Variables|Default|GetRespawnLocation) false false)
  (Variables|Default|SetisDeath false)
  (Components|Activation|SetActive (Variables|Character|GetCharacterMovement) true false)
  (Variables|Default|SetHealth 1e+02)
  (Default|CallChangingHealth (/ (Variables|Default|GetHealth) (Variables|Default|GetMaxHealth))))

(event Game|Damage|EventAnyDamage
  (params (Damage :type Float%20%28single-precision%29) (DamageType :type Damage%20Type%20Object%20Reference) (InstigatedBy :type Controller%20Object%20Reference) (DamageCauser :type Actor%20Object%20Reference))
  (if (not (Variables|Default|GetisDeath))
    (Variables|Default|SetHealth (- (Variables|Default|GetHealth) Damage))
    (Development|PrintString (Utilities|String|Append "Health: " (Utilities|String|ToString(Float) (Variables|Default|GetHealth))))
    (Default|CallChangingHealth (/ (Variables|Default|GetHealth) (Variables|Default|GetMaxHealth)))
    (if (> (Variables|Default|GetHealth) 0.0)
      (Math|Float|CompareFloat (.x (Transformation|GetWorldLocation (Variables|Default|GetSprite))) (Variables|Default|GetEnemyPositionX)
        (:>
          (Character|LaunchCharacter "500.000000, 0, 0" true false))
        (:<
          (Character|LaunchCharacter "-500.000000, 0, 0" true false)))
      (else
        (Variables|Default|SetisDeath true)
        (Components|Activation|SetActive (Variables|Character|GetCharacterMovement) false false)
        (CallFunction|Respawn)))))

(event EventBeginPlay
  (Variables|Default|SetRespawnLocation (Transformation|GetActorLocation))
  (bind _asplayer_controller (Utilities|Casting|CastToPlayerController (Pawn|GetController)))
  (bind _returnvalue (UserInterface|CreateWidget "/Game/BluePrints/Hero/HUD/W_HealthBar.W_HealthBar_C" _asplayer_controller))
  (UserInterface|Viewport|AddtoViewport _returnvalue 0)
  (Variables|Default|SetHealth 1e+02)
  (Default|CallChangingHealth (/ (Variables|Default|GetHealth) (Variables|Default|GetMaxHealth))))

(event EventOnJumped
  (Variables|Default|SetJumpMaxCount 2)
  (Class|PaperZDAnimInstance|JumptoNode (Variables|/Script/PaperZD.PaperZDAnimationComponent|GetAnimInstance (Variables|Default|GetAnimationComponent)) "JumpAction" "None"))

(event EventOnWalkingOffLedge
  (params (PreviousFloorImpactNormal :type Vector%20%28by%20ref%29 :default "0, 0, 0") (PreviousFloorContactNormal :type Vector%20%28by%20ref%29 :default "0, 0, 0") (PreviousLocation :type Vector%20%28by%20ref%29 :default "0, 0, 0") (TimeDelta :type Float%20%28single-precision%29))
  (Class|PaperZDAnimInstance|JumptoNode (Variables|/Script/PaperZD.PaperZDAnimationComponent|GetAnimInstance (Variables|Default|GetAnimationComponent)) "JumpAction" "None"))

(event EventOnLanded
  (params (Hit :type Hit%20Result%20Structure%20%28by%20ref%29))
  (Class|PaperZDAnimInstance|JumptoNode (Variables|/Script/PaperZD.PaperZDAnimationComponent|GetAnimInstance (Variables|Default|GetAnimationComponent)) "Landed" "None")
  (Components|Movement|StopMovementImmediately (Variables|Character|GetCharacterMovement))
  (Variables|Default|SetIsMovementLock true))

(event EventTick
  (params (DeltaSeconds :type Float%20%28single-precision%29))
  (bind _returnvalue (Pawn|GetController))
  (bind _returnvalue_2 (Pawn|GetController))
  (if (not (Variables|Default|GetIsMovementLock))
    (Math|Float|CompareFloat (.x (Variables|/Script/Engine.MovementComponent|GetVelocity (Variables|Character|GetCharacterMovement))) 0.0
      (:>
        (Utilities|IsValid _returnvalue_2
          (:Is%20Valid
            (Pawn|SetControlRotation _returnvalue_2 (Math|Rotator|MakeRotator 0.0 0.0 0.0)))))
      (:<
        (Utilities|IsValid _returnvalue
          (:Is%20Valid
            (Pawn|SetControlRotation _returnvalue (Math|Rotator|MakeRotator 0.0 0.0 1.8e+02))))))))

(event Input|ActionEvents|InputActionDash
  (params (Key :type Key%20Structure :default "None"))
  (:Pressed
    (Variables|Default|SetRunPlayRate 1.5)
    (Variables|/Script/Engine.CharacterMovementComponent|SetMaxWalkSpeed (Variables|Character|GetCharacterMovement) 8e+02))
  (:Released
    (Variables|Default|SetRunPlayRate 1.0)
    (Variables|/Script/Engine.CharacterMovementComponent|SetMaxWalkSpeed (Variables|Character|GetCharacterMovement) 4e+02)))

(event Input|ActionEvents|InputActionJump
  (params (Key :type Key%20Structure :default "None"))
  (:Pressed
    (Variables|Default|SetJumpMaxCount 2)
    (Variables|Default|SetJumpMaxHoldTime 0.1)
    (Character|Jump))
  (:Released
    (Character|StopJumping)))

(event Input|ActionEvents|InputActionBasicAttack
  (params (Key :type Key%20Structure :default "None"))
  (:Pressed
    (if (and (not (Variables|Default|GetisAttacking)) (AI|Components|NavMovement|IsMovingonGround (Variables|Character|GetCharacterMovement)))
      (Variables|Default|SetisAttacking true)
      (Class|PaperZDAnimInstance|JumptoNode (Variables|/Script/PaperZD.PaperZDAnimationComponent|GetAnimInstance (Variables|Default|GetAnimationComponent)) "BasicAttack" "None")
      (Components|Movement|StopMovementImmediately (Variables|Character|GetCharacterMovement))
      (Variables|Default|SetIsMovementLock true)
      (Utilities|FlowControl|Delay 0.5)
      (Variables|Default|SetisAttacking false))))

(event Input|ActionEvents|InputActionHeavyAttack
  (params (Key :type Key%20Structure :default "None"))
  (:Pressed
    (if (and (not (Variables|Default|GetisAttacking)) (AI|Components|NavMovement|IsMovingonGround (Variables|Character|GetCharacterMovement)))
      (Variables|Default|SetisAttacking true)
      (Class|PaperZDAnimInstance|JumptoNode (Variables|/Script/PaperZD.PaperZDAnimationComponent|GetAnimInstance (Variables|Default|GetAnimationComponent)) "HeavyAttack" "None")
      (Components|Movement|StopMovementImmediately (Variables|Character|GetCharacterMovement))
      (Variables|Default|SetIsMovementLock true)
      (Utilities|FlowControl|Delay 0.7)
      (Variables|Default|SetisAttacking false))))

(event Input|ActionEvents|InputActionRangeAttack
  (params (Key :type Key%20Structure :default "None"))
  (bind _sprite (Variables|Default|GetSprite))
  (bind _returnvalue (Transformation|GetWorldTransform _sprite))
  (:Pressed
    (Utilities|FlowControl|Delay 0.6)
    (Audio|PlaySound2D "/Game/Assets/Thunder/Sounds/Storage_bin.Storage_bin" 1.0 1.0 0.0 0 0)
    (Variables|Default|SetIsMovementLock true)
    (Class|PaperZDAnimInstance|JumptoNode (Variables|/Script/PaperZD.PaperZDAnimationComponent|GetAnimInstance (Variables|Default|GetAnimationComponent)) "RangeAttack" "None")
    (Utilities|FlowControl|Delay 0.1)
    (Game|SpawnActorfromClass "/Game/BluePrints/Hero/BP_Thunder.BP_Thunder_C" (Math|Transform|MakeTransform (Math|Vector|MakeVector (.x (.location _returnvalue)) (.y (.location _returnvalue)) (+ (.z (.location _returnvalue)) 1e+02)) (.rotation _returnvalue) (.scale _returnvalue)) "Undefined" 0 0)))

(event Input|AxisEvents|InputAxisMoveming
  (params (AxisValue :type Float%20%28single-precision%29))
  (if (not (Variables|Default|GetIsMovementLock))
    (Pawn|Input|AddMovementInput "0.700000,0.000000, 0" AxisValue false)))

(fn ConstructionScript)