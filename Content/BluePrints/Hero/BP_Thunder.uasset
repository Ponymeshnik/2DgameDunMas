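; BP_Thunder is a hero projectile that deals fixed damage to an actor overlapping its box collider.
; On overlap with any actor other than itself, it plays a hit sound, applies damage and stops its projectile movement, zeroing gravity.
; It then hides the projectile visual, shows a non-looping hit animation and destroys itself after a short delay.
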(event OnComponentBeginOverlap(Box)
  (params (OverlappedComponent :type Primitive%20Component%20Object%20Reference) (OtherActor :type Actor%20Object%20Reference) (OtherComp :type Primitive%20Component%20Object%20Reference) (OtherBodyIndex :type Integer) (bFromSweep :type Boolean) (SweepResult :type Hit%20Result%20Structure%20%28by%20ref%29))
  (bind _projectilemovement (Variables|Default|GetProjectileMovement))
  (bind _bp_hit (Variables|Default|GetBP_Hit))
  (if (!= OtherActor self)
    (Audio|PlaySound2D "/Game/Assets/Thunder/Sounds/Sonic_Pulse_Hit_02.Sonic_Pulse_Hit_02" 1.0 1.0 0.0 0 0)
    (Game|Damage|ApplyDamage OtherActor 7e+01 0 0)
    (Rendering|SetVisibility (Variables|Default|GetBP_ProjectTile) false false)
    (Variables|/Script/Engine.ProjectileMovementComponent|SetProjectileGravityScale _projectilemovement 0.0)
    (Components|Movement|StopMovementImmediately _projectilemovement)
    (Rendering|SetVisibility _bp_hit true false)
    (Components|Timeline|SetPlayRate _bp_hit 1.0)
    (Components|Timeline|SetLooping _bp_hit false)
    (Utilities|FlowControl|Delay 0.35)
    (Actor|DestroyActor)))

(event EventBeginPlay)

(event Collision|EventActorBeginOverlap
  (params (OtherActor :type Actor%20Object%20Reference)))

(event EventTick
  (params (DeltaSeconds :type Float%20%28single-precision%29)))

(fn ConstructionScript)